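; HUD for The Last Room, a first-person escape-room puzzle, drawn in immediate mode with hardcoded Ukrainian text.
; DrawHUD branches on the BP_FirstPerson Mode value to show exploration overlay, note, book and clock clues, keypad, victory banner or intro screen.
; Exploration shows an interact prompt when Focus is above zero, and the keypad displays the character's Code and Status.
; It only draws rects and text at viewport-relative offsets, with no input handling.
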(event `self.ReceiveDrawHUD`
  (params (SizeX :type Integer) (SizeY :type Integer))
  (bind _returnvalue (* (`KismetMathLibrary.Conv_IntToDouble` SizeX) 0.5))
  (bind _returnvalue_2 (* (`KismetMathLibrary.Conv_IntToDouble` SizeY) 0.5))
  (bind _asbp_first_person (cast `/Game/Blueprints/BP_FirstPerson` (`GameplayStatics.GetPlayerCharacter` 0) :!pure true))
  (if (== (`/Game/Blueprints/BP_FirstPerson.Mode` _asbp_first_person) 0)
    (`self.DrawRect` (struct :`R` 0.91 :`G` 0.88 :`B` 0.79 :`A` 1) (+ _returnvalue -2.0) (+ _returnvalue_2 -2.0) 4.0 4.0)
    (`self.DrawText` "THE LAST ROOM" (struct :`R` 0.91 :`G` 0.88 :`B` 0.79 :`A` 1) 36.0 28.0 "/Engine/EngineFonts/Roboto.Roboto" 0.85)
    (`self.DrawText` "ДОСЛІДІТЬ КІМНАТУ · ЗНАЙДІТЬ ВИХІД" (struct :`R` 0.48 :`G` 0.58 :`B` 0.58 :`A` 1) 36.0 54.0 "/Engine/EngineFonts/Roboto.Roboto" 0.65)
    (`self.DrawText` "WASD  рух    Миша  огляд    Пробіл  стрибок    E / ЛКМ  взаємодія" (struct :`R` 0.91 :`G` 0.88 :`B` 0.79 :`A` 1) 36.0 (+ (`KismetMathLibrary.Conv_IntToDouble` SizeY) -42.0) "/Engine/EngineFonts/Roboto.Roboto" 0.75)
    (if (> (`/Game/Blueprints/BP_FirstPerson.Focus` _asbp_first_person) 0)
      (`self.DrawRect` (struct :`R` 0.012 :`G` 0.025 :`B` 0.028 :`A` 0.97) (+ _returnvalue -195.0) (+ (`KismetMathLibrary.Conv_IntToDouble` SizeY) -114.0) 390.0 44.0)
      (`self.DrawText` "[ E ]   Натисніть E, щоб взаємодіяти" (struct :`R` 0.91 :`G` 0.88 :`B` 0.79 :`A` 1) (+ _returnvalue -177.0) (+ (`KismetMathLibrary.Conv_IntToDouble` SizeY) -102.0) "/Engine/EngineFonts/Roboto.Roboto" 0.85))
    (elif (== (`/Game/Blueprints/BP_FirstPerson.Mode` _asbp_first_person) 1)
      (`self.DrawRect` (struct :`R` 0.012 :`G` 0.025 :`B` 0.028 :`A` 0.97) (+ _returnvalue -280.0) (+ _returnvalue_2 -300.0) 560.0 600.0)
      (`self.DrawRect` (struct :`R` 0.96 :`G` 0.61 :`B` 0.23 :`A` 1) (+ _returnvalue -280.0) (+ _returnvalue_2 -300.0) 3.0 600.0)
      (`self.DrawText` "01  /  ПЕРША ПІДКАЗКА" (struct :`R` 0.96 :`G` 0.61 :`B` 0.23 :`A` 1) (+ _returnvalue -244.0) (+ _returnvalue_2 -265.0) "/Engine/EngineFonts/Roboto.Roboto" 0.85)
      (`self.DrawText` "Записка на столі" (struct :`R` 0.91 :`G` 0.88 :`B` 0.79 :`A` 1) (+ _returnvalue -244.0) (+ _returnvalue_2 -229.0) "/Engine/EngineFonts/Roboto.Roboto" 1.7)
      (`self.DrawText` "«У цій кімнаті час не рухається." (struct :`R` 0.91 :`G` 0.88 :`B` 0.79 :`A` 1) (+ _returnvalue -242.0) (+ _returnvalue_2 -145.0) "/Engine/EngineFonts/Roboto.Roboto" 0.97)
      (`self.DrawText` "Та він досі пам’ятає шлях назовні." (struct :`R` 0.91 :`G` 0.88 :`B` 0.79 :`A` 1) (+ _returnvalue -242.0) (+ _returnvalue_2 -110.0) "/Engine/EngineFonts/Roboto.Roboto" 0.97)
      (`self.DrawText` "Погляньте на годинник." (struct :`R` 0.91 :`G` 0.88 :`B` 0.79 :`A` 1) (+ _returnvalue -242.0) (+ _returnvalue_2 -50.0) "/Engine/EngineFonts/Roboto.Roboto" 0.97)
      (`self.DrawText` "Порядок цифр знайдете у книзі VIII." (struct :`R` 0.91 :`G` 0.88 :`B` 0.79 :`A` 1) (+ _returnvalue -242.0) (+ _returnvalue_2 -15.0) "/Engine/EngineFonts/Roboto.Roboto" 0.97)
      (`self.DrawText` "Не всі початки помітні з першого погляду»." (struct :`R` 0.91 :`G` 0.88 :`B` 0.79 :`A` 1) (+ _returnvalue -242.0) (+ _returnvalue_2 65.0) "/Engine/EngineFonts/Roboto.Roboto" 0.97)
      (`self.DrawText` "ЛКМ / Esc — повернутися" (struct :`R` 0.48 :`G` 0.58 :`B` 0.58 :`A` 1) (+ _returnvalue -242.0) (+ _returnvalue_2 248.0) "/Engine/EngineFonts/Roboto.Roboto" 0.8)
      (elif (== (`/Game/Blueprints/BP_FirstPerson.Mode` _asbp_first_person) 2)
        (`self.DrawRect` (struct :`R` 0.012 :`G` 0.025 :`B` 0.028 :`A` 0.97) (+ _returnvalue -280.0) (+ _returnvalue_2 -300.0) 560.0 600.0)
        (`self.DrawRect` (struct :`R` 0.96 :`G` 0.61 :`B` 0.23 :`A` 1) (+ _returnvalue -280.0) (+ _returnvalue_2 -300.0) 3.0 600.0)
        (`self.DrawText` "02  /  АРХІВ СПОСТЕРЕЖЕНЬ" (struct :`R` 0.96 :`G` 0.61 :`B` 0.23 :`A` 1) (+ _returnvalue -244.0) (+ _returnvalue_2 -265.0) "/Engine/EngineFonts/Roboto.Roboto" 0.85)
        (`self.DrawText` "Книга VIII · Про час" (struct :`R` 0.91 :`G` 0.88 :`B` 0.79 :`A` 1) (+ _returnvalue -244.0) (+ _returnvalue_2 -229.0) "/Engine/EngineFonts/Roboto.Roboto" 1.7)
        (`self.DrawText` "«Години завжди йдуть першими." (struct :`R` 0.91 :`G` 0.88 :`B` 0.79 :`A` 1) (+ _returnvalue -242.0) (+ _returnvalue_2 -145.0) "/Engine/EngineFonts/Roboto.Roboto" 0.95)
        (`self.DrawText` "Хвилини завершують послідовність." (struct :`R` 0.91 :`G` 0.88 :`B` 0.79 :`A` 1) (+ _returnvalue -242.0) (+ _returnvalue_2 -110.0) "/Engine/EngineFonts/Roboto.Roboto" 0.95)
        (`self.DrawText` "Кожній частині належать дві цифри." (struct :`R` 0.91 :`G` 0.88 :`B` 0.79 :`A` 1) (+ _returnvalue -242.0) (+ _returnvalue_2 -45.0) "/Engine/EngineFonts/Roboto.Roboto" 0.95)
        (`self.DrawText` "Якщо цифра одна — перед нею стоїть нуль»." (struct :`R` 0.91 :`G` 0.88 :`B` 0.79 :`A` 1) (+ _returnvalue -242.0) (+ _returnvalue_2 -10.0) "/Engine/EngineFonts/Roboto.Roboto" 0.95)
        (`self.DrawText` "ГГ  →  ХХ" (struct :`R` 0.96 :`G` 0.61 :`B` 0.23 :`A` 1) (+ _returnvalue -242.0) (+ _returnvalue_2 75.0) "/Engine/EngineFonts/Roboto.Roboto" 1.5)
        (`self.DrawText` "ЛКМ / Esc — повернутися" (struct :`R` 0.48 :`G` 0.58 :`B` 0.58 :`A` 1) (+ _returnvalue -242.0) (+ _returnvalue_2 248.0) "/Engine/EngineFonts/Roboto.Roboto" 0.8)
        (elif (== (`/Game/Blueprints/BP_FirstPerson.Mode` _asbp_first_person) 3)
          (`self.DrawRect` (struct :`R` 0.012 :`G` 0.025 :`B` 0.028 :`A` 0.97) (+ _returnvalue -280.0) (+ _returnvalue_2 -300.0) 560.0 600.0)
          (`self.DrawRect` (struct :`R` 0.96 :`G` 0.61 :`B` 0.23 :`A` 1) (+ _returnvalue -280.0) (+ _returnvalue_2 -300.0) 3.0 600.0)
          (`self.DrawText` "03  /  ВИХІД ЗАБЛОКОВАНО" (struct :`R` 0.96 :`G` 0.61 :`B` 0.23 :`A` 1) (+ _returnvalue -244.0) (+ _returnvalue_2 -265.0) "/Engine/EngineFonts/Roboto.Roboto" 0.85)
          (`self.DrawText` "Кодовий замок" (struct :`R` 0.91 :`G` 0.88 :`B` 0.79 :`A` 1) (+ _returnvalue -244.0) (+ _returnvalue_2 -229.0) "/Engine/EngineFonts/Roboto.Roboto" 1.7)
          (`self.DrawRect` (struct :`R` ".04" :`G` ".09" :`B` ".09" :`A` 1) (+ _returnvalue -164.0) (+ _returnvalue_2 -168.0) 328.0 52.0)
          (`self.DrawText` (`/Game/Blueprints/BP_FirstPerson.Code` _asbp_first_person) (struct :`R` 0.96 :`G` 0.61 :`B` 0.23 :`A` 1) (+ _returnvalue -140.0) (+ _returnvalue_2 -161.0) "/Engine/EngineFonts/Roboto.Roboto" 1.6)
          (`self.DrawRect` (struct :`R` ".07" :`G` ".12" :`B` ".13" :`A` 1) (+ _returnvalue -164.0) (+ _returnvalue_2 -95.0) 104.0 62.0)
          (`self.DrawText` "1" (struct :`R` 0.91 :`G` 0.88 :`B` 0.79 :`A` 1) (+ _returnvalue -125.0) (+ _returnvalue_2 -81.0) "/Engine/EngineFonts/Roboto.Roboto" 1.3)
          (`self.DrawRect` (struct :`R` ".07" :`G` ".12" :`B` ".13" :`A` 1) (+ _returnvalue -52.0) (+ _returnvalue_2 -95.0) 104.0 62.0)
          (`self.DrawText` "2" (struct :`R` 0.91 :`G` 0.88 :`B` 0.79 :`A` 1) (+ _returnvalue -13.0) (+ _returnvalue_2 -81.0) "/Engine/EngineFonts/Roboto.Roboto" 1.3)
          (`self.DrawRect` (struct :`R` ".07" :`G` ".12" :`B` ".13" :`A` 1) (+ _returnvalue 60.0) (+ _returnvalue_2 -95.0) 104.0 62.0)
          (`self.DrawText` "3" (struct :`R` 0.91 :`G` 0.88 :`B` 0.79 :`A` 1) (+ _returnvalue 99.0) (+ _returnvalue_2 -81.0) "/Engine/EngineFonts/Roboto.Roboto" 1.3)
          (`self.DrawRect` (struct :`R` ".07" :`G` ".12" :`B` ".13" :`A` 1) (+ _returnvalue -164.0) (+ _returnvalue_2 -25.0) 104.0 62.0)
          (`self.DrawText` "4" (struct :`R` 0.91 :`G` 0.88 :`B` 0.79 :`A` 1) (+ _returnvalue -125.0) (+ _returnvalue_2 -11.0) "/Engine/EngineFonts/Roboto.Roboto" 1.3)
          (`self.DrawRect` (struct :`R` ".07" :`G` ".12" :`B` ".13" :`A` 1) (+ _returnvalue -52.0) (+ _returnvalue_2 -25.0) 104.0 62.0)
          (`self.DrawText` "5" (struct :`R` 0.91 :`G` 0.88 :`B` 0.79 :`A` 1) (+ _returnvalue -13.0) (+ _returnvalue_2 -11.0) "/Engine/EngineFonts/Roboto.Roboto" 1.3)
          (`self.DrawRect` (struct :`R` ".07" :`G` ".12" :`B` ".13" :`A` 1) (+ _returnvalue 60.0) (+ _returnvalue_2 -25.0) 104.0 62.0)
          (`self.DrawText` "6" (struct :`R` 0.91 :`G` 0.88 :`B` 0.79 :`A` 1) (+ _returnvalue 99.0) (+ _returnvalue_2 -11.0) "/Engine/EngineFonts/Roboto.Roboto" 1.3)
          (`self.DrawRect` (struct :`R` ".07" :`G` ".12" :`B` ".13" :`A` 1) (+ _returnvalue -164.0) (+ _returnvalue_2 45.0) 104.0 62.0)
          (`self.DrawText` "7" (struct :`R` 0.91 :`G` 0.88 :`B` 0.79 :`A` 1) (+ _returnvalue -125.0) (+ _returnvalue_2 59.0) "/Engine/EngineFonts/Roboto.Roboto" 1.3)
          (`self.DrawRect` (struct :`R` ".07" :`G` ".12" :`B` ".13" :`A` 1) (+ _returnvalue -52.0) (+ _returnvalue_2 45.0) 104.0 62.0)
          (`self.DrawText` "8" (struct :`R` 0.91 :`G` 0.88 :`B` 0.79 :`A` 1) (+ _returnvalue -13.0) (+ _returnvalue_2 59.0) "/Engine/EngineFonts/Roboto.Roboto" 1.3)
          (`self.DrawRect` (struct :`R` ".07" :`G` ".12" :`B` ".13" :`A` 1) (+ _returnvalue 60.0) (+ _returnvalue_2 45.0) 104.0 62.0)
          (`self.DrawText` "9" (struct :`R` 0.91 :`G` 0.88 :`B` 0.79 :`A` 1) (+ _returnvalue 99.0) (+ _returnvalue_2 59.0) "/Engine/EngineFonts/Roboto.Roboto" 1.3)
          (`self.DrawRect` (struct :`R` ".07" :`G` ".12" :`B` ".13" :`A` 1) (+ _returnvalue -164.0) (+ _returnvalue_2 115.0) 104.0 62.0)
          (`self.DrawText` "C" (struct :`R` 0.91 :`G` 0.88 :`B` 0.79 :`A` 1) (+ _returnvalue -125.0) (+ _returnvalue_2 129.0) "/Engine/EngineFonts/Roboto.Roboto" 1.3)
          (`self.DrawRect` (struct :`R` ".07" :`G` ".12" :`B` ".13" :`A` 1) (+ _returnvalue -52.0) (+ _returnvalue_2 115.0) 104.0 62.0)
          (`self.DrawText` "0" (struct :`R` 0.91 :`G` 0.88 :`B` 0.79 :`A` 1) (+ _returnvalue -13.0) (+ _returnvalue_2 129.0) "/Engine/EngineFonts/Roboto.Roboto" 1.3)
          (`self.DrawRect` (struct :`R` ".07" :`G` ".12" :`B` ".13" :`A` 1) (+ _returnvalue 60.0) (+ _returnvalue_2 115.0) 104.0 62.0)
          (`self.DrawText` "OK" (struct :`R` 0.96 :`G` 0.61 :`B` 0.23 :`A` 1) (+ _returnvalue 99.0) (+ _returnvalue_2 129.0) "/Engine/EngineFonts/Roboto.Roboto" 1.3)
          (`self.DrawText` (`/Game/Blueprints/BP_FirstPerson.Status` _asbp_first_person) (struct :`R` 0.96 :`G` 0.61 :`B` 0.23 :`A` 1) (+ _returnvalue -242.0) (+ _returnvalue_2 199.0) "/Engine/EngineFonts/Roboto.Roboto" 0.8)
          (`self.DrawText` "Цифри / ЛКМ · Enter — OK · Backspace · Esc — назад" (struct :`R` 0.48 :`G` 0.58 :`B` 0.58 :`A` 1) (+ _returnvalue -242.0) (+ _returnvalue_2 260.0) "/Engine/EngineFonts/Roboto.Roboto" 0.7)
          (elif (== (`/Game/Blueprints/BP_FirstPerson.Mode` _asbp_first_person) 4)
            (`self.DrawRect` (struct :`R` 0.012 :`G` 0.025 :`B` 0.028 :`A` 0.97) (+ _returnvalue -300.0) 35.0 600.0 160.0)
            (`self.DrawText` "ВИХІД ВІДКРИТО" (struct :`R` 0.96 :`G` 0.61 :`B` 0.23 :`A` 1) (+ _returnvalue -228.0) 56.0 "/Engine/EngineFonts/Roboto.Roboto" 1.8)
            (`self.DrawText` "Ви розгадали таємницю останньої кімнати." (struct :`R` 0.91 :`G` 0.88 :`B` 0.79 :`A` 1) (+ _returnvalue -228.0) 111.0 "/Engine/EngineFonts/Roboto.Roboto" 0.95)
            (`self.DrawText` "R / ЛКМ — почати знову" (struct :`R` 0.48 :`G` 0.58 :`B` 0.58 :`A` 1) (+ _returnvalue -228.0) 153.0 "/Engine/EngineFonts/Roboto.Roboto" 0.8)
            (elif (== (`/Game/Blueprints/BP_FirstPerson.Mode` _asbp_first_person) 5)
              (`self.DrawRect` (struct :`R` 0.012 :`G` 0.025 :`B` 0.028 :`A` 0.97) (+ _returnvalue -280.0) (+ _returnvalue_2 -300.0) 560.0 600.0)
              (`self.DrawRect` (struct :`R` 0.96 :`G` 0.61 :`B` 0.23 :`A` 1) (+ _returnvalue -280.0) (+ _returnvalue_2 -300.0) 3.0 600.0)
              (`self.DrawText` "СПОСТЕРЕЖЕННЯ  /  ЧАС" (struct :`R` 0.96 :`G` 0.61 :`B` 0.23 :`A` 1) (+ _returnvalue -244.0) (+ _returnvalue_2 -265.0) "/Engine/EngineFonts/Roboto.Roboto" 0.85)
              (`self.DrawText` "Зупинений годинник" (struct :`R` 0.91 :`G` 0.88 :`B` 0.79 :`A` 1) (+ _returnvalue -244.0) (+ _returnvalue_2 -229.0) "/Engine/EngineFonts/Roboto.Roboto" 1.7)
              (`self.DrawText` "Коротка стрілка — трохи після восьмої." (struct :`R` 0.91 :`G` 0.88 :`B` 0.79 :`A` 1) (+ _returnvalue -242.0) (+ _returnvalue_2 -125.0) "/Engine/EngineFonts/Roboto.Roboto" 0.95)
              (`self.DrawText` "Довга стрілка — на п’ятій поділці." (struct :`R` 0.91 :`G` 0.88 :`B` 0.79 :`A` 1) (+ _returnvalue -242.0) (+ _returnvalue_2 -85.0) "/Engine/EngineFonts/Roboto.Roboto" 0.95)
              (`self.DrawText` "08 : 25" (struct :`R` 0.96 :`G` 0.61 :`B` 0.23 :`A` 1) (+ _returnvalue -242.0) (+ _returnvalue_2 10.0) "/Engine/EngineFonts/Roboto.Roboto" 2.8)
              (`self.DrawText` "ЛКМ / Esc — повернутися" (struct :`R` 0.48 :`G` 0.58 :`B` 0.58 :`A` 1) (+ _returnvalue -242.0) (+ _returnvalue_2 248.0) "/Engine/EngineFonts/Roboto.Roboto" 0.8)
              (elif (== (`/Game/Blueprints/BP_FirstPerson.Mode` _asbp_first_person) 6)
                (`self.DrawRect` (struct :`R` 0.012 :`G` 0.025 :`B` 0.028 :`A` 0.97) (+ _returnvalue -280.0) (+ _returnvalue_2 -300.0) 560.0 600.0)
                (`self.DrawRect` (struct :`R` 0.96 :`G` 0.61 :`B` 0.23 :`A` 1) (+ _returnvalue -280.0) (+ _returnvalue_2 -300.0) 3.0 600.0)
                (`self.DrawText` "НЕВЕЛИКА ІСТОРІЯ ПРО ВТЕЧУ" (struct :`R` 0.96 :`G` 0.61 :`B` 0.23 :`A` 1) (+ _returnvalue -244.0) (+ _returnvalue_2 -265.0) "/Engine/EngineFonts/Roboto.Roboto" 0.85)
                (`self.DrawText` "THE LAST ROOM" (struct :`R` 0.91 :`G` 0.88 :`B` 0.79 :`A` 1) (+ _returnvalue -244.0) (+ _returnvalue_2 -229.0) "/Engine/EngineFonts/Roboto.Roboto" 1.7)
                (`self.DrawText` "Одна кімната. Три підказки. Один вихід." (struct :`R` 0.91 :`G` 0.88 :`B` 0.79 :`A` 1) (+ _returnvalue -242.0) (+ _returnvalue_2 -142.0) "/Engine/EngineFonts/Roboto.Roboto" 0.95)
                (`self.DrawText` "Дослідіть стіл, книжкову шафу та годинник." (struct :`R` 0.91 :`G` 0.88 :`B` 0.79 :`A` 1) (+ _returnvalue -242.0) (+ _returnvalue_2 -80.0) "/Engine/EngineFonts/Roboto.Roboto" 0.95)
                (`self.DrawText` "Знайдіть чотири цифри й відчиніть двері." (struct :`R` 0.91 :`G` 0.88 :`B` 0.79 :`A` 1) (+ _returnvalue -242.0) (+ _returnvalue_2 -45.0) "/Engine/EngineFonts/Roboto.Roboto" 0.95)
                (`self.DrawText` "WASD — рух     Миша — огляд" (struct :`R` 0.48 :`G` 0.58 :`B` 0.58 :`A` 1) (+ _returnvalue -242.0) (+ _returnvalue_2 38.0) "/Engine/EngineFonts/Roboto.Roboto" 0.9)
                (`self.DrawText` "Пробіл — стрибок     E / ЛКМ — взаємодія" (struct :`R` 0.48 :`G` 0.58 :`B` 0.58 :`A` 1) (+ _returnvalue -242.0) (+ _returnvalue_2 73.0) "/Engine/EngineFonts/Roboto.Roboto" 0.9)
                (`self.DrawRect` (struct :`R` ".15" :`G` ".22" :`B` ".21" :`A` 1) (+ _returnvalue -242.0) (+ _returnvalue_2 170.0) 484.0 58.0)
                (`self.DrawText` "НАТИСНІТЬ ЛКМ, ЩОБ ПОЧАТИ" (struct :`R` 0.96 :`G` 0.61 :`B` 0.23 :`A` 1) (+ _returnvalue -215.0) (+ _returnvalue_2 187.0) "/Engine/EngineFonts/Roboto.Roboto" 0.95)))))))))

(fn `UserConstructionScript`)